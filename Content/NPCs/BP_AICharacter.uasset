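; Wandering NPC that the player can talk to, given a random walk speed at spawn.
; WalkEvent loops AIMoveTo to random navigable points, pausing randomly after success or failure.
; Box overlap sets AIOverlap on the ThirdPersonCharacter and a greeting; leaving clears both, restores speed and hides the dialogue widget.
; TalkEvent, not called within this graph, halts movement and shows random dialogue lines in all top-level AICharacter_DialogueWidgets.
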(event OnComponentBeginOverlap(Box)
  (params (OverlappedComponent :type Primitive%20Component%20Object%20Reference) (OtherActor :type Actor%20Object%20Reference) (OtherComp :type Primitive%20Component%20Object%20Reference) (OtherBodyIndex :type Integer) (bFromSweep :type Boolean) (SweepResult :type Hit%20Result%20Structure%20%28by%20ref%29))
  ;[1 1 1] Overlap Logic
  (bind _asthird_person_character (Utilities|Casting|CastToThirdPersonCharacter OtherActor))
  (Variables|/Game/Utils/ThirdPersonBP/Blueprints/ThirdPersonCharacter.ThirdPersonCharacter_C|SetAI%20Overlap _asthird_person_character true)
  (Variables|Default|SetDialogue "Hello"))

(event OnComponentEndOverlap(Box)
  (params (OverlappedComponent :type Primitive%20Component%20Object%20Reference) (OtherActor :type Actor%20Object%20Reference) (OtherComp :type Primitive%20Component%20Object%20Reference) (OtherBodyIndex :type Integer))
  ;[1 1 1] Overlap Logic
  (bind _asthird_person_character (Utilities|Casting|CastToThirdPersonCharacter OtherActor))
  (Variables|/Game/Utils/ThirdPersonBP/Blueprints/ThirdPersonCharacter.ThirdPersonCharacter_C|SetAI%20Overlap _asthird_person_character false)
  (Variables|Default|SetDialogue "")
  (Variables|Default|SetIs%20Talking false)
  (Variables|/Script/Engine.CharacterMovementComponent|SetMaxWalkSpeed (Variables|Character|GetCharacterMovement) (Variables|Default|GetWalk_Speed))
  (Widget|SetVisibility (stale Custom|TalkEvent _array_element) "Hidden"))

(event Custom|Walk%20Event
  ;[1 1 1] Walk Login
  (if (not (Variables|Default|GetWalking?))
    (AI|AIMoveTo self (.RandomLocation (Class|NavigationSystem|GetRandomPointinNavigableRadius (Transformation|GetActorLocation) (Variables|Default|GetWalk_Radius))) 0 5.0 false
      (:then
        (Variables|Default|SetWalking? true))
      (:OnSuccess
        (Utilities|FlowControl|Delay (Math|Random|RandomFloatinRange 1.0 5.0) :!label _label)
        (Variables|Default|SetWalking? false)
        (CallFunction|WalkEvent))
      (:OnFail
        (goto _label)))))

(event Custom|TalkEvent
  (bind _adialoguelines (Variables|Default|GetaDialogueLines))
  (Variables|/Script/Engine.CharacterMovementComponent|SetMaxWalkSpeed (Variables|Character|GetCharacterMovement) 0.0)
  (bind _foundwidgets (Widget|GetAllWidgetsOfClass "/Game/NPCs/AICharacter_DialogueWidget.AICharacter_DialogueWidget_C" true))
  (for _array_element _foundwidgets
    (if true
      (Variables|/Game/NPCs/AICharacter_DialogueWidget.AICharacter_DialogueWidget_C|SetDialogue _array_element (Utilities|Array|Get(acopy) _adialoguelines (Math|Random|RandomIntegerinRange 0 (Utilities|Array|LastIndex _adialoguelines))))
      (Widget|SetVisibility _array_element "Visible"))))

(event EventBeginPlay
  ;[1 1 1] Walk Login
  (bind _output_get (Variables|Default|SetWalk_Speed (Math|Random|RandomFloatinRange 1e+02 4.5e+02)))
  (Variables|/Script/Engine.CharacterMovementComponent|SetMaxWalkSpeed (Variables|Character|GetCharacterMovement) _output_get)
  (CallFunction|WalkEvent))

(fn ConstructionScript)