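; BP_AIGrandpaJack is the AI Blueprint for the Grandpa Jack NPC, with logic for random wandering.
; WalkEvent moves it to random navigable points within WalkRadius, looping after a random pause on success or failure, gated by a Walking flag.
; MoveToLocations instead heads for a stored target point.
; The nodes that set that target, randomize walk speed and start wandering are disconnected, so nothing here starts the loop.
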(event Custom|Walk%20Event
  ;[1 1 1] Walk Logic
  (if (not (Variables|Default|GetWalking?))
    (AI|AIMoveTo self (.RandomLocation (Class|NavigationSystem|GetRandomPointinNavigableRadius (Transformation|GetActorLocation) (Variables|Default|GetWalk_Radius))) 0 5.0 false
      (:then
        (Variables|Default|SetWalking? true))
      (:OnSuccess
        (Utilities|FlowControl|Delay (Math|Random|RandomFloatinRange 1.0 5.0) :!label _label)
        (Variables|Default|SetWalking? false)
        (CallFunction|WalkEvent))
      (:OnFail
        (goto _label)))))

(event Custom|MoveToLocations
  (if (not (Variables|Default|GetWalking?))
    (AI|Navigation|SimpleMovetoLocation (Pawn|GetController) (Transformation|GetActorLocation (stale _astarget_point)))))

(fn ConstructionScript)